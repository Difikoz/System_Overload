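; AC_Health is a health component that tracks a current value against a maximum and a dead state.
; Reduce and restore clamp the value between zero and Max, then broadcast OnValueChanged.
; Reaching zero through damage latches IsDead, which blocks further changes, and each function returns whether the owner is dead.
; Regenerate feeds a delta-time-scaled rate into RestoreCurrent, so it cannot revive the dead.
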(fn ReduceCurrent
  (params (Value :type Float%20%28double-precision%29))
  (if (Variables|Default|GetIsDead)
    (return true)
    (else
      (bind _output_get (Variables|Default|SetCurrent (Math|Float|Clamp(Float) (- (Variables|Default|GetCurrent) Value) 0.0 (Variables|Default|GetMax))))
      (Default|CallOnValueChanged _output_get (Variables|Default|GetMax))
      (if (> _output_get 0.0)
        (return false)
        (else
          (Variables|Default|SetIsDead true)
          (return true))))))

(fn RestoreCurrent
  (params (Value :type Float%20%28double-precision%29))
  (if (Variables|Default|GetIsDead)
    (return true)
    (else
      (bind _output_get (Variables|Default|SetCurrent (Math|Float|Clamp(Float) (+ Value (Variables|Default|GetCurrent)) 0.0 (Variables|Default|GetMax))))
      (Default|CallOnValueChanged _output_get (Variables|Default|GetMax))
      (return false))))

(fn Regenerate
  (params (DeltaTime :type Float%20%28double-precision%29))
  (bind _died (CallFunction|RestoreCurrent (* DeltaTime (Variables|Default|GetRegeneration))))
  (return _died))