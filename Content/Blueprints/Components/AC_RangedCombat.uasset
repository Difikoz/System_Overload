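; Ranged combat component that gives its owner hitscan weapon fire with a fire-rate limit.
; Fire line-traces on Visibility from a socket on the owner's weapon mesh along its forward vector, drawing debug lines, and applies damage on a hit.
; A CanFire gate reopens after a delay of one over FireSpeed.
; Initialize stores the owner; the component's own ApplyDamage function is an empty stub.
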(event Custom|Initialize
  (params (Owner :type BP%20Character%20Object%20Reference))
  (Variables|References|SetOwner Owner))

(event Custom|Fire
  (bind _owner (Variables|References|GetOwner))
  (bind _tracepointname (Variables|Default|GetTracePointName))
  (bind _skm_weapon (Variables|/Game/Blueprints/Characters/BP_Character.BP_Character_C|GetSKM_Weapon _owner))
  (bind _returnvalue (Transformation|GetSocketLocation _skm_weapon _tracepointname))
  (if (Variables|Default|GetCanFire)
    (Variables|Default|SetCanFire false)
    (bind (_outhit _returnvalue_2) (Collision|LineTraceByChannel _returnvalue (+ _returnvalue (* (Math|Vector|GetForwardVector (Transformation|GetSocketRotation _skm_weapon (Variables|Default|GetTracePointName))) (Variables|Properties|GetTraceRange))) "TraceTypeQuery1" false 0 "ForDuration" true "(R=1.000000,G=0.000000,B=0.000000,A=1.000000)" "(R=0.000000,G=1.000000,B=0.000000,A=1.000000)" 0.25))
    (Utilities|FlowControl|Sequence
      (:then_0
        (if _returnvalue_2
          (Game|Damage|ApplyDamage (.HitActor (Collision|BreakHitResult _outhit)) (Variables|Properties|GetFireDamage) 0 (Variables|References|GetOwner))))
      (:then_1
        (Utilities|FlowControl|Delay (/ 1.0 (Variables|Properties|GetFireSpeed)))
        (Variables|Default|SetCanFire true)))))

(fn ApplyDamage
  (params (Target :type Object%20Object%20Reference)))