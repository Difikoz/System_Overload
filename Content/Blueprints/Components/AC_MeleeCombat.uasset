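; Melee combat component that gives its owner a three-hit, stamina-costed montage combo with weapon hit detection.
; Attack starts a swing or buffers input mid-attack; StartCombo consumes that buffer to play the next montage by AttackIndex, or resets the combo.
; StartTrace and StopTrace bracket a looping timer that debug-draws sphere traces between weapon sockets, applying damage while DamagedTargets blocks repeat hits until cleared by the next swing.
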(event Custom|Attack
  (if (Variables|Default|GetCanAttack)
    (if (Variables|Default|GetIsAttacking)
      (Variables|Default|SetDelayedAttack true)
      (else
        (Variables|Default|SetIsAttacking true)
        (bind _enough (Default|ReduceCurrent (Variables|/Game/Blueprints/Characters/BP_Character.BP_Character_C|GetAC_Stamina (Variables|References|GetOwner)) (Variables|Properties|GetAttackStaminaCost)))
        (if _enough
          (switch int (Variables|Default|GetAttackIndex)
            (:0
              (CallFunction|Combo1))
            (:1
              (CallFunction|Combo2))
            (:2
              (CallFunction|Combo3))))))))

(event Custom|StartTrace
  (bind _returnvalue (Utilities|Time|SetTimerbyEvent (delegate Custom|TraceLoop) (stale EventTick DeltaSeconds) true))
  (Variables|Default|SetTraceTimer _returnvalue))

(event Custom|Initialize
  (params (Owner :type BP%20Character%20Object%20Reference))
  (Variables|References|SetOwner Owner))

(event Custom|StartCombo
  (if (Variables|Default|GetDelayedAttack)
    (Variables|Default|SetDelayedAttack false)
    (bind _enough (Default|ReduceCurrent (Variables|/Game/Blueprints/Characters/BP_Character.BP_Character_C|GetAC_Stamina (Variables|References|GetOwner)) (Variables|Properties|GetAttackStaminaCost)))
    (if _enough
      (switch int (Variables|Default|GetAttackIndex)
        (:0
          (CallFunction|Combo1))
        (:1
          (CallFunction|Combo2))
        (:2
          (CallFunction|Combo3))))
    (else
      (CallFunction|StopCombo))))

(event Custom|StopCombo
  (Variables|Default|SetIsAttacking false)
  (Variables|Default|SetAttackIndex 0))

(event Custom|Combo%201
  (Utilities|FlowControl|DoOnce false :!label _label
    (:Completed
      (Utilities|FlowControl|Delay 0.2)
      (Animation|Montage|PlayMontage (Variables|/Script/Engine.Character|GetMesh (Variables|References|GetOwner)) "/Game/Models/Characters/Mannequins/Animations/Manny/Montages/Attack_1_Montage.Attack_1_Montage"
        (:then
          (Variables|Default|SetAttackIndex 1)
          (Utilities|Array|Clear (Variables|Default|GetDamagedTargets))
          (goto _label Reset))))))

(event Custom|Combo%202
  (Utilities|FlowControl|DoOnce false :!label _label
    (:Completed
      (Utilities|FlowControl|Delay 0.2)
      (Animation|Montage|PlayMontage (Variables|/Script/Engine.Character|GetMesh (Variables|References|GetOwner)) "/Game/Models/Characters/Mannequins/Animations/Manny/Montages/Attack_2_Montage.Attack_2_Montage"
        (:then
          (Variables|Default|SetAttackIndex 2)
          (Utilities|Array|Clear (Variables|Default|GetDamagedTargets))
          (goto _label Reset))))))

(event Custom|Combo%203
  (Utilities|FlowControl|DoOnce false :!label _label
    (:Completed
      (Utilities|FlowControl|Delay 0.2)
      (Animation|Montage|PlayMontage (Variables|/Script/Engine.Character|GetMesh (Variables|References|GetOwner)) "/Game/Models/Characters/Mannequins/Animations/Manny/Montages/Attack_3_Montage.Attack_3_Montage"
        (:then
          (Variables|Default|SetAttackIndex 3)
          (Utilities|Array|Clear (Variables|Default|GetDamagedTargets))
          (goto _label Reset))))))

(event Custom|TraceLoop
  (bind _owner (Variables|References|GetOwner))
  (bind _skm_weapon (Variables|/Game/Blueprints/Characters/BP_Character.BP_Character_C|GetSKM_Weapon _owner))
  (bind (_outhit _returnvalue) (Collision|SphereTraceByChannel (Transformation|GetSocketLocation _skm_weapon "TraceStartPoint") (Transformation|GetSocketLocation _skm_weapon "TraceEndPoint") (Variables|Properties|GetTraceRadius) "TraceTypeQuery1" false 0 "ForDuration" true "(R=1.000000,G=0.000000,B=0.000000,A=1.000000)" "(R=0.000000,G=1.000000,B=0.000000,A=1.000000)" 0.5))
  (if _returnvalue
    (if (not (Utilities|Array|ContainsItem (Variables|Default|GetDamagedTargets) (.HitActor (Collision|BreakHitResult _outhit))))
      (Game|Damage|ApplyDamage (.HitActor (Collision|BreakHitResult _outhit)) (Variables|Properties|GetAttackDamage) 0 (Variables|References|GetOwner))
      (Utilities|Array|Add (Variables|Default|GetDamagedTargets) (.HitActor (Collision|BreakHitResult _outhit))))))

(event Custom|StopTrace
  (Utilities|Time|ClearandInvalidateTimerbyHandle (Variables|Default|GetTraceTimer)))

(event EventTick
  (params (DeltaSeconds :type Float%20%28single-precision%29)))