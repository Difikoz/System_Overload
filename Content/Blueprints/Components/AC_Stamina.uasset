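; AC_Stamina is a component that tracks a stamina value between zero and a maximum.
; ReduceCurrent spends stamina only when enough is available and returns whether it succeeded, while RestoreCurrent adds stamina up to the maximum.
; Both clamp the value and fire an OnValueChanged event with current and max values.
; Regenerate restores stamina at a per-second rate scaled by delta time.
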(fn ReduceCurrent
  (params (Value :type Float%20%28double-precision%29))
  (if (>= (Variables|Default|GetCurrent) Value)
    (bind _output_get (Variables|Default|SetCurrent (Math|Float|Clamp(Float) (- (Variables|Default|GetCurrent) Value) 0.0 (Variables|Default|GetMax))))
    (Default|CallOnValueChanged _output_get (Variables|Default|GetMax))
    (return true)
    (else
      (return false))))

(fn RestoreCurrent
  (params (Value :type Float%20%28double-precision%29))
  (bind _output_get (Variables|Default|SetCurrent (Math|Float|Clamp(Float) (+ Value (Variables|Default|GetCurrent)) 0.0 (Variables|Default|GetMax))))
  (Default|CallOnValueChanged _output_get (Variables|Default|GetMax))
  (return))

(fn Regenerate
  (params (DeltaTime :type Float%20%28double-precision%29))
  (CallFunction|RestoreCurrent (* DeltaTime (Variables|Default|GetRegeneration))))