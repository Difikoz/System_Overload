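; AC_Experience is a component that tracks experience points and level for its owner.
; AddExperience adds to Current, then loops while it meets Required, calling LevelUp, subtracting the unchanged threshold and broadcasting OnValueChanged only on those level-up passes.
; LevelUp increments Level one step at a time, firing OnLevelChanged for each step.
; ForceUpdate rebroadcasts both values on demand.
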(fn AddExperience
  (params (Value :type Integer))
  (Variables|Default|SetCurrent (+ Value (Variables|Default|GetCurrent)))
  (if (>= (Variables|Default|GetCurrent) (Variables|Default|GetRequired)) :!label _label
    (CallFunction|LevelUp 1)
    (bind _output_get (Variables|Default|SetCurrent (- (Variables|Default|GetCurrent) (Variables|Default|GetRequired))))
    (Default|CallOnValueChanged _output_get (Variables|Default|GetRequired))
    (goto _label)
    (else
      (return))))

(fn LevelUp
  (params (Amount :type Integer))
  (if (> Amount 0) :!label _label
    (bind _result (Math|Integer|IncrementInt (Variables|Default|GetLevel))
      (:%20%20
        (Math|Integer|DecrementInt Amount
          (:%20%20
            (Default|CallOnLevelChanged _result)
            (goto _label)))))
    (else
      (return))))

(fn ForceUpdate
  (Default|CallOnValueChanged (Variables|Default|GetCurrent) (Variables|Default|GetRequired))
  (Default|CallOnLevelChanged (Variables|Default|GetLevel))
  (return))