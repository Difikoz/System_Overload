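; Player-style character Blueprint with health, stamina, melee and ranged combat components, hit reactions and ragdoll death.
; Input events drive movement, timeline-blended sprint and crouch, and attacks that fire when aiming or swing melee otherwise.
; Jump, sprint and melee are stamina-gated, while health and stamina regenerate each tick.
; Jumping runs trace-based vault detection, then either plays a motion-warped vault montage with collision disabled or jumps normally.
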(event Custom|Die
  (Physics|SetSimulatePhysics (Variables|Character|GetMesh) true))

(event EventTick
  (params (DeltaSeconds :type Float%20%28single-precision%29))
  (CallFunction|Regeneration DeltaSeconds)
  (CallFunction|CalculateMoveMagnitude))

(event EventBeginPlay
  (Default|Initialize (Variables|Default|GetAC_MeleeCombat) self)
  (Default|Initialize (Variables|Default|GetAC_RangedCombat) self)
  (CallFunction|StopSprinting))

(event Game|Damage|EventAnyDamage
  (params (Damage :type Float%20%28single-precision%29) (DamageType :type Damage%20Type%20Object%20Reference) (InstigatedBy :type Controller%20Object%20Reference) (DamageCauser :type Actor%20Object%20Reference))
  (bind _hitreacts (Variables|Default|GetHitReacts))
  (if (not (Variables|/Game/Blueprints/Components/AC_Health.AC_Health_C|GetIsDead (Variables|Default|GetAC_Health)))
    (bind _died (Default|ReduceCurrent (Variables|Default|GetAC_Health) Damage))
    (if _died
      (CallFunction|Die)
      (else
        (Animation|PlayAnimMontage (Utilities|Array|Get(acopy) _hitreacts (Math|Random|RandomIntegerinRange 0 (Utilities|Array|Length _hitreacts))) 1.0 "None")))))

(fn ConstructionScript)

(fn CalculateMoveMagnitude
  (bind _charactermovement (Variables|Character|GetCharacterMovement))
  (bind _velocity (Variables|/Script/Engine.MovementComponent|GetVelocity _charactermovement))
  (bind _returnvalue (Math|Vector|VectorLengthXY _velocity))
  (switch Utilities|FlowControl|Switch|SwitchonEnum_MovementState (Variables|Movement|GetMovementState)
    (:NewEnumerator0
      (Variables|Movement|SetMoveMagnitude (/ _returnvalue (Variables|Standing|GetWalkSpeed))))
    (:NewEnumerator1
      (Variables|Movement|SetMoveMagnitude (Utilities|Operators|Divide _returnvalue (Variables|Standing|GetSprintSpeed) 0.5)))
    (:NewEnumerator2
      (Variables|Movement|SetMoveMagnitude (/ _returnvalue (Variables|Crouching|GetCrouchSpeed)))))
  (return))

(fn VaultCheck
  (LocalVariables|SetVaultSuccess false)
  (bind _index (Utilities|FlowControl|ForLoopwithBreak 0 (LocalVariables|GetMaxUpTraceStepCount) :!label _label)
    (:LoopBody
      (bind (_outhit _returnvalue) (Collision|SphereTraceByChannel (+ (Transformation|GetActorLocation) (Math|Vector|MakeVector 0.0 0.0 (* _index (LocalVariables|GetMaxUpTraceStepDistance)))) (+ (+ (Transformation|GetActorLocation) (Math|Vector|MakeVector 0.0 0.0 (* _index (LocalVariables|GetMaxUpTraceStepDistance)))) (* (Math|Vector|GetForwardVector (Transformation|GetActorRotation)) (Variables|Vaulting|GetVaultDistance))) 5.0 "TraceTypeQuery1" false 0 "ForDuration" true "(R=1.000000,G=0.000000,B=0.000000,A=1.000000)" "(R=0.000000,G=1.000000,B=0.000000,A=1.000000)" 0.5))
      (if _returnvalue
        (Utilities|FlowControl|Sequence
          (:then_0
            (goto _label Break))
          (:then_1
            (bind _index_2 (Utilities|FlowControl|ForLoopwithBreak 0 (LocalVariables|GetMaxForwardTraceStepCount) :!label _label_2)
              (:LoopBody
                (bind (_outhit_2 _returnvalue_2) (Collision|SphereTraceByChannel (+ (* (* _index_2 (LocalVariables|GetMaxForwardTraceStepDistance)) (Math|Vector|GetForwardVector (Transformation|GetActorRotation))) (+ (.Location (Collision|BreakHitResult _outhit)) (Math|Vector|MakeVector 0.0 0.0 (LocalVariables|GetHeightCheckOffset)))) (- (+ (* (* _index_2 (LocalVariables|GetMaxForwardTraceStepDistance)) (Math|Vector|GetForwardVector (Transformation|GetActorRotation))) (+ (.Location (Collision|BreakHitResult _outhit)) (Math|Vector|MakeVector 0.0 0.0 (LocalVariables|GetHeightCheckOffset)))) (Math|Vector|MakeVector 0.0 0.0 (LocalVariables|GetHeightCheckOffset))) 1e+01 "TraceTypeQuery1" false 0 "ForDuration" true "(R=1.000000,G=0.000000,B=0.000000,A=1.000000)" "(R=0.000000,G=1.000000,B=0.000000,A=1.000000)" 0.5))
                (if _returnvalue_2
                  (Utilities|FlowControl|Sequence
                    (:then_0
                      (if (== _index_2 0)
                        (Variables|Vaulting|SetVaultStartPosition (.Location (Collision|BreakHitResult _outhit_2)))))
                    (:then_1
                      (Variables|Vaulting|SetVaultMiddlePosition (.Location (Collision|BreakHitResult _outhit_2)))
                      (Variables|Default|SetCanWarp true)))
                  (else
                    (bind (_outhit_3 _returnvalue_3) (Collision|LineTraceByChannel (+ (.TraceStart (Collision|BreakHitResult _outhit_2)) (* (Math|Vector|GetForwardVector (Transformation|GetActorRotation)) (LocalVariables|GetMaxEndDistance))) (- (+ (.TraceStart (Collision|BreakHitResult _outhit_2)) (* (Math|Vector|GetForwardVector (Transformation|GetActorRotation)) (LocalVariables|GetMaxEndDistance))) (Math|Vector|MakeVector 0.0 0.0 (LocalVariables|GetMaxFallHeight))) "TraceTypeQuery1" false 0 "ForDuration" true "(R=1.000000,G=0.000000,B=0.000000,A=1.000000)" "(R=0.000000,G=1.000000,B=0.000000,A=1.000000)" 0.5))
                    (if _returnvalue_3
                      (Variables|Vaulting|SetVaultEndPosition (.Location (Collision|BreakHitResult _outhit_3)))
                      (LocalVariables|SetVaultSuccess true)
                      (goto _label_2 Break)))))
              (:Completed
                (return (LocalVariables|GetVaultSuccess))))))))
    (:Completed
      (return false))))

(fn Regeneration
  (params (DeltaTime :type Float%20%28double-precision%29))
  (if (Variables|/Game/Blueprints/Components/AC_Health.AC_Health_C|GetIsDead (Variables|Default|GetAC_Health))
    (return)
    (else
      (Default|Regenerate (Variables|Default|GetAC_Health) DeltaTime)
      (Default|Regenerate (Variables|Default|GetAC_Stamina) DeltaTime (> (Variables|Movement|GetMoveMagnitude) 0.0) (Variables|Standing|GetIsSpringting))
      (return))))

(event Custom|LookInput
  (params (Horizontal :type Float%20%28single-precision%29) (Vertical :type Float%20%28double-precision%29))
  (Pawn|Input|AddControllerYawInput Horizontal)
  (Pawn|Input|AddControllerPitchInput Vertical))

(event Custom|MoveInput
  (params (Horizontal :type Float%20%28double-precision%29) (Vertical :type Float%20%28double-precision%29))
  (bind _returnvalue (Pawn|GetControlRotation :!class /Script/Engine.Pawn))
  (Pawn|Input|AddMovementInput (Math|Vector|GetRightVector (Math|Rotator|MakeRotator (.roll _returnvalue) 0.0 (.yaw _returnvalue))) Horizontal false)
  (Pawn|Input|AddMovementInput (Math|Vector|GetForwardVector (Math|Rotator|MakeRotator 0.0 0.0 (.yaw (Pawn|GetControlRotation :!class /Script/Engine.Pawn)))) Vertical false))

(event Custom|StartVaultMotionWarp
  (Variables|Vaulting|SetIsVaulting true)
  (Pawn|Components|CharacterMovement|SetMovementMode (Variables|Character|GetCharacterMovement) "MOVE_Flying" 0)
  (Collision|SetActorEnableCollision false)
  (Class|MotionWarpingComponent|AddorUpdateWarpTarget (Variables|Default|GetMotionWarping) (Utilities|Struct|MakeMotionWarpingTarget "VaultStart" (Variables|Vaulting|GetVaultStartPosition) (Transformation|GetActorRotation) 0 "None" false "0.000000,0.000000,0.000000" "0.000000,0.000000,0.000000"))
  (Class|MotionWarpingComponent|AddorUpdateWarpTarget (Variables|Default|GetMotionWarping) (Utilities|Struct|MakeMotionWarpingTarget "VaultMiddle" (Variables|Vaulting|GetVaultMiddlePosition) (Transformation|GetActorRotation) 0 "None" false "0.000000,0.000000,0.000000" "0.000000,0.000000,0.000000"))
  (Class|MotionWarpingComponent|AddorUpdateWarpTarget (Variables|Default|GetMotionWarping) (Utilities|Struct|MakeMotionWarpingTarget "VaultEnd" (Variables|Vaulting|GetVaultEndPosition) (Transformation|GetActorRotation) 0 "None" false "0.000000,0.000000,0.000000" "0.000000,0.000000,0.000000"))
  (Animation|Montage|PlayMontage (Variables|Character|GetMesh) "/Game/Models/Characters/Mannequins/Animations/Manny/Montages/Vault_Over_Montage.Vault_Over_Montage"
    (:OnCompleted
      (Pawn|Components|CharacterMovement|SetMovementMode (Variables|Character|GetCharacterMovement) "MOVE_Walking" 0)
      (Collision|SetActorEnableCollision true)
      (Variables|Default|SetCanWarp false)
      (Variables|Vaulting|SetVaultEndPosition "0.000000,0.000000,999999.000000")
      (Variables|Vaulting|SetIsVaulting false))))

(event Custom|ToggleJump
  (params (Apply :type Boolean))
  (bind _charactermovement (Variables|Character|GetCharacterMovement))
  (bind _mesh (Variables|Character|GetMesh))
  (bind _returnvalue (Transformation|GetWorldLocation _mesh))
  (if Apply
    (if (not (Math|Boolean|ORBoolean (Variables|/Game/Blueprints/Components/AC_MeleeCombat.AC_MeleeCombat_C|GetIsAttacking (Variables|Default|GetAC_MeleeCombat)) (Variables|Vaulting|GetIsVaulting) (Utilities|Enum|Equal(Enum) (Variables|/Script/Engine.CharacterMovementComponent|GetMovementMode (Variables|Character|GetCharacterMovement)) "MOVE_Falling")))
      (if (>= (Variables|/Game/Blueprints/Components/AC_Stamina.AC_Stamina_C|GetCurrent (Variables|Default|GetAC_Stamina)) (Variables|Stamina|GetJumpStaminaCost))
        (if (Variables|Crouching|GetIsCrouching)
          (CallFunction|StopCrouching)
          (Utilities|FlowControl|Delay 0.25)
          (if (not (Variables|Crouching|GetIsCrouching))
            (Variables|/Script/Engine.CharacterMovementComponent|SetJumpZVelocity _charactermovement (Variables|Crouching|GetCrouchJumpHeight))
            (bind _enough (Default|ReduceCurrent (Variables|Default|GetAC_Stamina) (Variables|Stamina|GetJumpStaminaCost) :!label _label))
            (if _enough
              (bind _vaulted (CallFunction|VaultCheck))
              (if (Math|Boolean|ANDBoolean _vaulted (Variables|Default|GetCanWarp) (Math|Float|InRange(Float) (.z (Variables|Vaulting|GetVaultEndPosition)) (- (.z _returnvalue) 1e+02) (+ (.z _returnvalue) 1e+02)))
                (CallFunction|StartVaultMotionWarp)
                (else
                  (Character|Jump)))))
          (else
            (Variables|/Script/Engine.CharacterMovementComponent|SetJumpZVelocity _charactermovement (Variables|Standing|GetStandJumpHeight))
            (goto _label)))))
    (else
      (Character|StopJumping))))

(event Custom|StartCrouching
  (if (Variables|Standing|GetIsSpringting)
    (CallFunction|StopSprinting)
    (Utilities|FlowControl|Delay 0.6)
    (if (not (Variables|Standing|GetIsSpringting))
      (Variables|Crouching|SetIsCrouching true :!label _label)
      (bind _time (Timeline|CrouchTimeline Play)
        (:Update
          (Components|Capsule|SetCapsuleHalfHeight (Variables|Collision|GetCapsuleComponent) (Math|Float|Lerp (Variables|Standing|GetStandHeight) (Variables|Crouching|GetCrouchHeight) _time) true)
          (Variables|/Script/Engine.CharacterMovementComponent|SetMaxWalkSpeed (Variables|Character|GetCharacterMovement) (Math|Float|Lerp (Variables|Standing|GetWalkSpeed) (Variables|Crouching|GetCrouchSpeed) _time)))
        (:Finished
          (if (Variables|Crouching|GetIsCrouching)
            (Variables|Movement|SetMovementState "NewEnumerator2")
            (else
              (Variables|Movement|SetMovementState "NewEnumerator0"))))))
    (else
      (goto _label))))

(event Custom|StopCrouching
  (bind _returnvalue (Transformation|GetActorLocation))
  (bind _capsulecomponent (Variables|Collision|GetCapsuleComponent))
  (bind _capsuleradius (Variables|/Script/Engine.CapsuleComponent|GetCapsuleRadius _capsulecomponent))
  (bind _returnvalue_2 (Collision|SphereTraceByChannel _returnvalue (+ _returnvalue (* (Transformation|GetActorUpVector) (- (Variables|Standing|GetStandHeight) _capsuleradius))) _capsuleradius "TraceTypeQuery1" false (Utilities|Array|MakeArray self) "ForDuration" true "(R=1.000000,G=0.000000,B=0.000000,A=1.000000)" "(R=0.000000,G=1.000000,B=0.000000,A=1.000000)" 0.5))
  (if (not _returnvalue_2)
    (Variables|Crouching|SetIsCrouching false)
    (bind _time (Timeline|CrouchTimeline Reverse)
      (:Update
        (Components|Capsule|SetCapsuleHalfHeight (Variables|Collision|GetCapsuleComponent) (Math|Float|Lerp (Variables|Standing|GetStandHeight) (Variables|Crouching|GetCrouchHeight) _time) true)
        (Variables|/Script/Engine.CharacterMovementComponent|SetMaxWalkSpeed (Variables|Character|GetCharacterMovement) (Math|Float|Lerp (Variables|Standing|GetWalkSpeed) (Variables|Crouching|GetCrouchSpeed) _time)))
      (:Finished
        (if (Variables|Crouching|GetIsCrouching)
          (Variables|Movement|SetMovementState "NewEnumerator2")
          (else
            (Variables|Movement|SetMovementState "NewEnumerator0")))))))

(event Custom|ToggleCrouch
  (if (Variables|Crouching|GetIsCrouching)
    (CallFunction|StopCrouching)
    (else
      (CallFunction|StartCrouching))))

(event Custom|StartSprinting
  (if (and (>= (Variables|/Game/Blueprints/Components/AC_Stamina.AC_Stamina_C|GetCurrent (Variables|Default|GetAC_Stamina)) (Variables|Stamina|GetSprintStaminaCost)) (> (Variables|Movement|GetMoveMagnitude) 0.0))
    (if (Variables|Crouching|GetIsCrouching)
      (CallFunction|StopCrouching)
      (Utilities|FlowControl|Delay 0.6)
      (if (not (Variables|Crouching|GetIsCrouching))
        (Variables|Standing|SetIsSpringting true :!label _label)
        (bind _time (Timeline|SprintTimeline Play)
          (:Update
            (Variables|/Script/Engine.CharacterMovementComponent|SetMaxWalkSpeed (Variables|Character|GetCharacterMovement) (Math|Float|Lerp (Variables|Standing|GetWalkSpeed) (Variables|Standing|GetSprintSpeed) _time)))
          (:Finished
            (if (Variables|Standing|GetIsSpringting)
              (Variables|Movement|SetMovementState "NewEnumerator1")
              (bind _returnvalue (Utilities|Time|SetTimerbyEvent (delegate Custom|ReduceStaminaBySprint) (Variables|Stamina|GetSprintStaminaDelay) true))
              (Variables|Stamina|SetSprintTimer _returnvalue)
              (else
                (Variables|Movement|SetMovementState "NewEnumerator0"))))))
      (else
        (goto _label)))))

(event Custom|StopSprinting
  (Utilities|Time|ClearandInvalidateTimerbyHandle (Variables|Stamina|GetSprintTimer))
  (Variables|Standing|SetIsSpringting false)
  (bind _time (Timeline|SprintTimeline Reverse)
    (:Update
      (Variables|/Script/Engine.CharacterMovementComponent|SetMaxWalkSpeed (Variables|Character|GetCharacterMovement) (Math|Float|Lerp (Variables|Standing|GetWalkSpeed) (Variables|Standing|GetSprintSpeed) _time)))
    (:Finished
      (if (Variables|Standing|GetIsSpringting)
        (Variables|Movement|SetMovementState "NewEnumerator1")
        (bind _returnvalue (Utilities|Time|SetTimerbyEvent (delegate Custom|ReduceStaminaBySprint) (Variables|Stamina|GetSprintStaminaDelay) true))
        (Variables|Stamina|SetSprintTimer _returnvalue)
        (else
          (Variables|Movement|SetMovementState "NewEnumerator0"))))))

(event Custom|ReduceStaminaBySprint
  (if (not (or (Utilities|Enum|Equal(Enum) (Variables|/Script/Engine.CharacterMovementComponent|GetMovementMode (Variables|Character|GetCharacterMovement)) "MOVE_Falling") (Variables|Vaulting|GetIsVaulting)))
    (bind _enough (Default|ReduceCurrent (Variables|Default|GetAC_Stamina) (* (Variables|Stamina|GetSprintStaminaCost) (Variables|Stamina|GetSprintStaminaDelay))))
    (if (not (and _enough (> (Variables|Movement|GetMoveMagnitude) 0.0)))
      (CallFunction|StopSprinting))))

(event Custom|ToggleSprint
  (if (Variables|Standing|GetIsSpringting)
    (CallFunction|StopSprinting)
    (else
      (CallFunction|StartSprinting))))

(event Custom|AttackInput
  (bind _ac_meleecombat (Variables|Default|GetAC_MeleeCombat))
  (if (not (or (Variables|Vaulting|GetIsVaulting) (Utilities|Enum|Equal(Enum) (Variables|/Script/Engine.CharacterMovementComponent|GetMovementMode (Variables|Character|GetCharacterMovement)) "MOVE_Falling")))
    (if (Variables|Combat|GetIsAiming)
      (Default|Fire (Variables|Default|GetAC_RangedCombat))
      (elif (>= (Variables|/Game/Blueprints/Components/AC_Stamina.AC_Stamina_C|GetCurrent (Variables|Default|GetAC_Stamina)) (Variables|/Game/Blueprints/Components/AC_MeleeCombat.AC_MeleeCombat_C|GetAttackStaminaCost _ac_meleecombat))
        (Default|Attack _ac_meleecombat)))))

(event Custom|AimInput
  (params (Aiming :type Boolean))
  (Variables|Combat|SetIsAiming Aiming))