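; Player character Blueprint that handles local input, HUD setup and death.
; On BeginPlay it adds the default Enhanced Input mapping context, creates and initializes the HUD widget, then force-updates the experience component.
; Input actions forward to movement, look, jump, sprint, crouch, attack and aim functions defined outside these graphs.
; Death disables input and enables physics simulation on the mesh for a ragdoll effect.
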(event Input|EnhancedActionEvents|EnhancedInputActionIA_Move
  (params (ActionValue :type Vector%202D%20Structure) (ElapsedSeconds :type Float%20%28double-precision%29) (TriggeredSeconds :type Float%20%28double-precision%29) (InputAction :type Input%20Action%20Object%20Reference :default "/Game/Input/Actions/IA_Move.IA_Move"))
  (CallFunction|MoveInput (.x ActionValue) (.y ActionValue)))

(event Input|EnhancedActionEvents|EnhancedInputActionIA_Look
  (params (ActionValue :type Vector%202D%20Structure) (ElapsedSeconds :type Float%20%28double-precision%29) (TriggeredSeconds :type Float%20%28double-precision%29) (InputAction :type Input%20Action%20Object%20Reference :default "/Game/Input/Actions/IA_Look.IA_Look"))
  (CallFunction|LookInput (.x ActionValue) (.y ActionValue)))

(event Input|EnhancedActionEvents|EnhancedInputActionIA_Jump
  (params (ActionValue :type Boolean) (ElapsedSeconds :type Float%20%28double-precision%29) (TriggeredSeconds :type Float%20%28double-precision%29) (InputAction :type Input%20Action%20Object%20Reference :default "/Game/Input/Actions/IA_Jump.IA_Jump"))
  (:Started
    (CallFunction|ToggleJump true))
  (:Completed
    (CallFunction|ToggleJump false)))

(event Input|EnhancedActionEvents|EnhancedInputActionIA_Sprint
  (params (ActionValue :type Boolean) (ElapsedSeconds :type Float%20%28double-precision%29) (TriggeredSeconds :type Float%20%28double-precision%29) (InputAction :type Input%20Action%20Object%20Reference :default "/Game/Input/Actions/IA_Sprint.IA_Sprint"))
  (:Started
    (CallFunction|ToggleSprint)))

(event Input|EnhancedActionEvents|EnhancedInputActionIA_Crouch
  (params (ActionValue :type Boolean) (ElapsedSeconds :type Float%20%28double-precision%29) (TriggeredSeconds :type Float%20%28double-precision%29) (InputAction :type Input%20Action%20Object%20Reference :default "/Game/Input/Actions/IA_Crouch.IA_Crouch"))
  (:Started
    (CallFunction|ToggleCrouch)))

(event Input|EnhancedActionEvents|EnhancedInputActionIA_PrimaryAction
  (params (ActionValue :type Boolean) (ElapsedSeconds :type Float%20%28double-precision%29) (TriggeredSeconds :type Float%20%28double-precision%29) (InputAction :type Input%20Action%20Object%20Reference :default "/Game/Input/Actions/IA_PrimaryAction.IA_PrimaryAction"))
  (:Started
    (CallFunction|AttackInput)))

(event Input|EnhancedActionEvents|EnhancedInputActionIA_SecondaryAction
  (params (ActionValue :type Boolean) (ElapsedSeconds :type Float%20%28double-precision%29) (TriggeredSeconds :type Float%20%28double-precision%29) (InputAction :type Input%20Action%20Object%20Reference :default "/Game/Input/Actions/IA_SecondaryAction.IA_SecondaryAction"))
  (:Started
    (CallFunction|AimInput true))
  (:Completed
    (CallFunction|AimInput false)))

(event EventBeginPlay
  (|CallParentFunction)
  (Input|AddMappingContext (PlayerController|LocalPlayerSubsystems|GetEnhancedInputLocalPlayerSubsystem (Game|GetPlayerController 0)) "/Game/Input/IMC_Default.IMC_Default" 0 "(bIgnoreAllPressedKeysUntilRelease=True,bForceImmediately=False,bNotifyUserSettings=False)")
  (bind _returnvalue (UserInterface|CreateWidget "/Game/Blueprints/UI/WB_HUD.WB_HUD_C" (Game|GetPlayerController 0)))
  (bind _output_get (Variables|Components|SetHUD _returnvalue))
  (UserInterface|Viewport|AddtoViewport _output_get 0)
  (Default|Initialize _output_get self)
  (Default|ForceUpdate (Variables|Default|GetAC_Experience)))

(event EventTick
  (params (DeltaSeconds :type Float%20%28single-precision%29))
  (|CallParentFunction DeltaSeconds) ; This node is disabled and will not be called.\nDrag off pins to build functionality.
)

(event EventDie
  (Input|DisableInput 0)
  (Physics|SetSimulatePhysics (Variables|Character|GetMesh) true))

(fn ConstructionScript
  (|CallParentFunction))